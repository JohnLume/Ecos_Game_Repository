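; Game mode that runs the game flow from main menu through play to credits.
; BeginPlay shows a timed loading screen, starts menu music and points the camera at the main BP_Menu3D actor.
; StartGame teleports the player to the spawn transform, adds the progress widget and swaps music, while PauseMenu toggles pause with a video options widget.
; OBJComplete updates progress through a delayed DoOnce and shows timed credits when the completion count equals twenty.
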(event `self.ReceiveBeginPlay`
  (bind _returnvalue (`GameplayStatics.GetPlayerController` 0))
  ;[1 1 1] StartGame
  (bind _returnvalue_2 (`|CreateWidget` "/Game/1GAME/3D_Menu/Widgets/LoadingScreen.LoadingScreen_C" (`GameplayStatics.GetPlayerController` 0)))
  (`UserWidget.AddToViewport` _returnvalue_2 0)
  (`|ExecutionSequence`
    (:`then_0`
      (`KismetSystemLibrary.Delay` 10.0)
      (`Widget.RemoveFromParent` _returnvalue_2))
    (:`then_1`
      (`KismetSystemLibrary.Delay` 8.0)
      (bind _returnvalue_3 (`GameplayStatics.SpawnSound2D` "/Game/1GAME/Sound/OST/OST_Menu.OST_Menu" 0.5 1.0 0.0 null false false))
      (set `self.MenuOST` _returnvalue_3)
      (bind _outactors (`GameplayStatics.GetAllActorsOfClass` "/Game/1GAME/3D_Menu/BP_Menu3D.BP_Menu3D_C"))
      (for _array_element _outactors
        (if (`/Game/1GAME/3D_Menu/BP_Menu3D.IsMainMenu` _array_element)
          (set `PlayerController.bShowMouseCursor` true _returnvalue)
          (`PlayerController.SetViewTargetWithBlend` _returnvalue _array_element 0.0 "VTBlend_Linear" 0.0 false)
          (`WidgetBlueprintLibrary.SetInputMode_GameAndUIEx` _returnvalue null "LockInFullscreen" false))))))

(event `StartGame`
  (bind _returnvalue (`GameplayStatics.GetPlayerController` 0))
  (bind _returnvalue_2 (`GameplayStatics.GetPlayerCharacter` 0))
  (bind _spawn_transform_location (`KismetMathLibrary.BreakTransform` (`self.Spawn Transform`)))
  (bind _menuost (`self.MenuOST`))
  ;[1 1 1] StartGame
  (bind _returnvalue_3 (`|CreateWidget` "/Game/1GAME/3D_Menu/WidgetProgresso.WidgetProgresso_C" (`GameplayStatics.GetPlayerController` 0)))
  (bind _output_get (set `self.ProgressUI` _returnvalue_3))
  (`UserWidget.AddToViewport` _output_get 0)
  (`self.K2_SetActorLocation` _returnvalue_2 _spawn_transform_location false true)
  (`PlayerController.SetViewTargetWithBlend` _returnvalue _returnvalue_2 0.0 "VTBlend_Linear" 0.0 false)
  (`WidgetBlueprintLibrary.SetInputMode_GameOnly` _returnvalue)
  (set `Pawn.bUseControllerRotationYaw` true _returnvalue_2)
  (set `PlayerController.bShowMouseCursor` false _returnvalue)
  (`AudioComponent.Stop` _menuost)
  (`ActorComponent.K2_DestroyComponent` _menuost)
  (bind _returnvalue_4 (`GameplayStatics.SpawnSound2D` "/Game/1GAME/Sound/OST/OST_Game.OST_Game" 0.3 1.0 0.0 null false false))
  (set `self.Ost_Game` _returnvalue_4))

(event `PauseMenu`
  (bind _returnvalue (`GameplayStatics.GetPlayerController` 0))
  ;[1 1 1] Game Pause
  (`/Engine/EditorBlueprintResources/StandardMacros.IsValid` (`self.VideoMenuRef`)
    (:`Is Valid`
      _)
    (:`Is Not Valid`
      (bind _returnvalue_2 (`|CreateWidget` "/Game/1GAME/3D_Menu/VideoOptionsWidget.VideoOptionsWidget_C"))
      (bind _output_get (set `self.VideoMenuRef` _returnvalue_2))))
  (if (`GameplayStatics.IsGamePaused`)
    (`Widget.RemoveFromParent` _output_get)
    (`GameplayStatics.SetGamePaused` false)
    (if (not (`self.IsIn3DMenu?`))
      (set `PlayerController.bShowMouseCursor` false _returnvalue)
      (`WidgetBlueprintLibrary.SetInputMode_GameOnly` _returnvalue))
    (else
      (`UserWidget.AddToViewport` _output_get 0)
      (`GameplayStatics.SetGamePaused` true)
      (set `PlayerController.bShowMouseCursor` true _returnvalue)
      (`WidgetBlueprintLibrary.SetInputMode_GameAndUIEx` _returnvalue null "LockInFullscreen" false))))

(event `OBJComplete`
  ;[0 0.2767 1] Zerar
  (`/Engine/EditorBlueprintResources/StandardMacros.DoOnce` false :!label _label
    (:`Completed`
      (`KismetSystemLibrary.Delay` 1.0)
      (`|ExecutionSequence`
        (:`then_0`
          (if (== (`self.NComplete`) 20.0)
            (set `self.Zerou?` true)
            (`KismetSystemLibrary.Delay` 10.0)
            (bind _returnvalue (`|CreateWidget` "/Game/1GAME/3D_Menu/WidgetCredits.WidgetCredits_C" (`GameplayStatics.GetPlayerController` 0)))
            (bind _output_get (set `self.Credits` _returnvalue))
            (`UserWidget.AddToViewport` _output_get 0)
            (`KismetSystemLibrary.Delay` 15.0)
            (`Widget.RemoveFromParent` _output_get)))
        (:`then_1`
          (goto _label :!via `Reset`))
        (:`then_2`
          (`/Game/1GAME/3D_Menu/WidgetProgresso.Progressed` (`self.ProgressUI`)))))))

(fn `UserConstructionScript`)
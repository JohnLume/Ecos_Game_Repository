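; BP_PuzzleCamera is a camera actor that switches the player's view to itself and back, likely for puzzle sequences.
; CameraStart waits a second, disables character movement, then makes this camera the view target.
; CameraEnd restores walking and returns the view to BP_EcoCharacter.
; Both switches are wrapped in camera fade calls with no delay between them, so the fade-in immediately overrides the fade-out.
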(event `CameraStart`
  (bind _asplayer_controller (cast `PlayerController` (`GameplayStatics.GetPlayerController` 0)))
  (`KismetSystemLibrary.Delay` 1.0)
  (`CharacterMovementComponent.DisableMovement` (`Character.CharacterMovement` (`GameplayStatics.GetPlayerCharacter` 0)))
  (bind _playercameramanager (`PlayerController.PlayerCameraManager` _asplayer_controller))
  (`PlayerCameraManager.StartCameraFade` :`self` _playercameramanager :`ToAlpha` 1.0 :`Duration` 2.0)
  (`PlayerController.SetViewTargetWithBlend` _asplayer_controller (`ActorComponent.GetOwner` (`self.Camera`)) 0.0 "VTBlend_Linear" 0.0 false)
  (`PlayerCameraManager.StartCameraFade` :`self` _playercameramanager :`FromAlpha` 1.0 :`Duration` 0.5))

(event `CameraEnd`
  (bind _returnvalue (`GameplayStatics.GetPlayerController` 0))
  (bind _playercameramanager (`PlayerController.PlayerCameraManager` _returnvalue))
  (bind _asplayer_controller (cast `PlayerController` _returnvalue))
  (bind _asbp_eco_character (cast `/Game/1GAME/Character/BP_EcoCharacter` (`GameplayStatics.GetPlayerCharacter` 0)))
  (`CharacterMovementComponent.SetMovementMode` (`Character.CharacterMovement` _asbp_eco_character) "MOVE_Walking" 0)
  (`PlayerCameraManager.StartCameraFade` :`self` _playercameramanager :`ToAlpha` 1.0 :`Duration` 0.3)
  (`PlayerController.SetViewTargetWithBlend` _asplayer_controller _asbp_eco_character 0.0 "VTBlend_Linear" 0.0 false)
  (`PlayerCameraManager.StartCameraFade` :`self` _playercameramanager :`FromAlpha` 1.0 :`Duration` 0.5))

(fn `UserConstructionScript`)
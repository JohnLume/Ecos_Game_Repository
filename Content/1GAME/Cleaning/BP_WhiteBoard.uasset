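; Cleanable whiteboard actor that records strokes at given locations and snaps to fully clean once enough of it is covered.
; Draw stamps a dynamic marker material into a 512px render target, which feeds the board's material, and into a 2x2 copy.
; After a delay it reads the tiny copy as a cheap coverage check, logging bright-blue cells as clean.
; Two or more clean cells clear the main target to white.
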(event `self.ReceiveBeginPlay`
  ;[1 0.4775 0.5173] Material Set up
  (bind _returnvalue (`KismetMaterialLibrary.CreateDynamicMaterialInstance` null))
  (set `self.MatDyn_Marker` _returnvalue)
  (bind _returnvalue_2 (`KismetRenderingLibrary.CreateRenderTarget2D` 512 512))
  (bind _output_get (set `self.RT` _returnvalue_2))
  (bind _returnvalue_3 (`KismetRenderingLibrary.CreateRenderTarget2D` 2 2))
  (set `self.RTSmall` _returnvalue_3)
  (`KismetRenderingLibrary.ClearRenderTarget2D` _output_get)
  (`KismetRenderingLibrary.ClearRenderTarget2D` (`self.RTSmall`))
  (bind _returnvalue_4 (`KismetMaterialLibrary.CreateDynamicMaterialInstance` "/Game/1GAME/Cleaning/Mat_WhiteBoard.Mat_WhiteBoard"))
  (bind _output_get_2 (set `self.MatDyn_WhiteBoard` _returnvalue_4))
  (`MaterialInstanceDynamic.SetTextureParameterValue` _output_get_2 "RT_Color" (`self.RT`))
  (`PrimitiveComponent.SetMaterial` (`self.Board`) 0 (`self.MatDyn_WhiteBoard`)))

(event `Draw`
  (params (`Location to draw` :type "Vector2D Structure"))
  (bind _matdyn_marker (`self.MatDyn_Marker`))
  (bind _clean_cells (`self.Clean Cells`))
  ;[1 0.8113 0] Drawing
  (`MaterialInstanceDynamic.SetVectorParameterValue` _matdyn_marker "DrawLocation" (`KismetMathLibrary.Conv_VectorToLinearColor` (`KismetMathLibrary.Conv_Vector2DToVector` `Location to draw`)))
  (`KismetRenderingLibrary.DrawMaterialToRenderTarget` (`self.RT`) _matdyn_marker)
  (`KismetRenderingLibrary.DrawMaterialToRenderTarget` (`self.RTSmall`) _matdyn_marker)
  (`KismetSystemLibrary.Delay` 2.0)
  (bind _outsamples (`KismetRenderingLibrary.ReadRenderTarget` (`self.RTSmall`)))
  (for (_array_element _array_index) _outsamples
    (if (>= (`.B` (break `Color` _array_element)) 200)
      (`KismetArrayLibrary.Array_AddUnique` _clean_cells _array_index)
      (if (>= (`KismetArrayLibrary.Array_Length` _clean_cells) 2)
        (`KismetRenderingLibrary.ClearRenderTarget2D` (`self.RT`) (struct :`R` 1.0 :`G` 1.0 :`B` 1.0 :`A` 1.0))))))

(fn `UserConstructionScript`)
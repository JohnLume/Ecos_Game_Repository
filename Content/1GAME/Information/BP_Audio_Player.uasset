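; BP_Audio_Player is an interactable actor with a Telefone component that plays an audio dialogue with typed-out on-screen text.
; Overlap events register or unregister it with BP_EcoCharacter and toggle its button prompt.
; StartTalk creates an ECOwritter_Widget to write TextToSpeak and plays a 2D sound chosen by the Audio variable.
; A DoOnce blocks repeats until writing finishes and, after a short delay, the widget is removed.
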(event `self.ReceiveActorBeginOverlap`
  (params (OtherActor :type "Actor Object Reference"))
  (bind _asbp_eco_character (cast `/Game/1GAME/Character/BP_EcoCharacter` OtherActor))
  (message `/Game/1GAME/Character/BPI_Interaction.Interact` _asbp_eco_character true self "")
  (`SceneComponent.SetVisibility` (`self.ButtonText`) true false))

(event `self.ReceiveActorEndOverlap`
  (params (OtherActor :type "Actor Object Reference"))
  (bind _asbp_eco_character (cast `/Game/1GAME/Character/BP_EcoCharacter` OtherActor))
  (message `/Game/1GAME/Character/BPI_Interaction.Interact` _asbp_eco_character false self "")
  (`SceneComponent.SetVisibility` (`self.ButtonText`) false false))

(event `Start Talk`
  ;[1 0.1921 0] Dialogue 1
  (`/Engine/EditorBlueprintResources/StandardMacros.DoOnce` false :!label _label
    (:`Completed`
      (bind _returnvalue (`|CreateWidget` "/Game/1GAME/Information/ECOwritter_Widget.ECOwritter_Widget_C" (`GameplayStatics.GetPlayerController` 0) 24.0))
      (bind _output_get (set `self.Current WG` _returnvalue))
      (`UserWidget.AddToViewport` _output_get 0)
      (`/Game/1GAME/Information/ECOwritter_Widget.Write` _output_get (`self.Text To Speak`))
      (add `/Game/1GAME/Information/ECOwritter_Widget.FinishedWriting` _output_get (delegate `FinishWirte`))
      (switch `/Game/1GAME/Information/AudioToPlay` (`self.Audio`)
        (:`NewEnumerator0`
          (`GameplayStatics.PlaySound2D` null 1.0 1.0 0.0 null null))
        (:`NewEnumerator1`
          (`GameplayStatics.PlaySound2D` null 1.0 1.0 0.0 null null))))))

(event `FinishWirte`
  ;[1 0.1921 0] Dialogue 1
  (`KismetSystemLibrary.Delay` 4.0)
  (`Widget.RemoveFromParent` (`self.Current WG`))
  (`self.AllowNexttext`))

(event `AllowNexttext`
  ;[1 0.1921 0] Dialogue 1
  (goto _label :!via `Reset`))

(fn `Allow New Text`)

(fn `UserConstructionScript`)
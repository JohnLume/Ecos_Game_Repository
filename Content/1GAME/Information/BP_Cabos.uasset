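; BP_Cabos is a spline-driven environment actor for laying out cables, ropes, pipes, brickwork and roof tiles along an editable path.
; The construction script loops over every spline segment and switches on the CableList selection to add one spline mesh component per segment.
; Each variant has its own add-component node, with identical logic bending the piece between consecutive points using local-space locations and tangents.
; It has no runtime logic.
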(fn `UserConstructionScript`
  (bind _spline (`self.Spline`))
  (for _index (range (`SplineComponent.GetNumberOfSplineSegments` _spline))
    (switch `/Game/1GAME/Information/CableList` (`self.CableList`)
      (:`NewEnumerator0`
        ;[0.319 0.9302 1] Cabos
        (bind _returnvalue (`AddComponent|NODE_AddSplineMeshComponent-0`))
        (`/Engine/EditorBlueprintResources/StandardMacros.IsValid` _returnvalue
          (:`Is Valid`
            (bind (_location _tangent) (`SplineComponent.GetLocationAndTangentAtSplinePoint` _spline _index "Local"))
            (bind (_location_2 _tangent_2) (`SplineComponent.GetLocationAndTangentAtSplinePoint` _spline (+ _index 1) "Local"))
            (`SplineMeshComponent.SetStartAndEnd` _returnvalue _location _tangent _location_2 _tangent_2 true))))
      (:`NewEnumerator1`
        (bind _returnvalue_2 (`AddComponent|NODE_AddSplineMeshComponent-1`))
        (`/Engine/EditorBlueprintResources/StandardMacros.IsValid` _returnvalue_2
          (:`Is Valid`
            (`SplineMeshComponent.SetStartAndEnd` _returnvalue_2 _location _tangent _location_2 _tangent_2 true))))
      (:`NewEnumerator2`
        (bind _returnvalue_3 (`AddComponent|NODE_AddSplineMeshComponent-2`))
        (`/Engine/EditorBlueprintResources/StandardMacros.IsValid` _returnvalue_3
          (:`Is Valid`
            (`SplineMeshComponent.SetStartAndEnd` _returnvalue_3 _location _tangent _location_2 _tangent_2 true))))
      (:`NewEnumerator4`
        (bind _returnvalue_4 (`AddComponent|NODE_AddSplineMeshComponent-3`))
        (`/Engine/EditorBlueprintResources/StandardMacros.IsValid` _returnvalue_4
          (:`Is Valid`
            (`SplineMeshComponent.SetStartAndEnd` _returnvalue_4 _location _tangent _location_2 _tangent_2 true))))
      (:`NewEnumerator5`
        ;[1 1 1] tijolo
        (bind _returnvalue_5 (`AddComponent|NODE_AddSplineMeshComponent-4`))
        (`/Engine/EditorBlueprintResources/StandardMacros.IsValid` _returnvalue_5
          (:`Is Valid`
            (`SplineMeshComponent.SetStartAndEnd` _returnvalue_5 _location _tangent _location_2 _tangent_2 true))))
      (:`NewEnumerator6`
        (bind _returnvalue_6 (`AddComponent|NODE_AddSplineMeshComponent-5`))
        (`/Engine/EditorBlueprintResources/StandardMacros.IsValid` _returnvalue_6
          (:`Is Valid`
            (`SplineMeshComponent.SetStartAndEnd` _returnvalue_6 _location _tangent _location_2 _tangent_2 true))))
      (:`NewEnumerator7`
        ;[1 0.4849 0.4351] Telhas
        (bind _returnvalue_7 (`AddComponent|NODE_AddSplineMeshComponent-6`))
        (`/Engine/EditorBlueprintResources/StandardMacros.IsValid` _returnvalue_7
          (:`Is Valid`
            (`SplineMeshComponent.SetStartAndEnd` _returnvalue_7 _location _tangent _location_2 _tangent_2 true))))
      (:`NewEnumerator8`
        (bind _returnvalue_8 (`AddComponent|NODE_AddSplineMeshComponent-7`))
        (`/Engine/EditorBlueprintResources/StandardMacros.IsValid` _returnvalue_8
          (:`Is Valid`
            (`SplineMeshComponent.SetStartAndEnd` _returnvalue_8 _location _tangent _location_2 _tangent_2 true))))
      (:`NewEnumerator9`
        (bind _returnvalue_9 (`AddComponent|NODE_AddSplineMeshComponent-8`))
        (`/Engine/EditorBlueprintResources/StandardMacros.IsValid` _returnvalue_9
          (:`Is Valid`
            (`SplineMeshComponent.SetStartAndEnd` _returnvalue_9 _location _tangent _location_2 _tangent_2 true)))))))
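; Talkable villager NPC whose NPCList enum selects hat and material in the construction script, plus one of several hard-coded dialogues.
; Overlap shows a text prompt and notifies BP_EcoCharacter; leaving ends the talk and resets the order.
; NPCTalk advances per-character MultiGates through SetNextText, displaying each line in a new ECOwritter_Widget typewriter while a gesture animation loops.
; Finishing the Fazendeiro dialogue also briefly triggers a matching BP_PuzzleCamera shot.
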(event `ResetWritter`
  ;[1 0.05967 0.1294] Display Dialogue
  (if (not (`self.Finished`))
    (`|ExecutionSequence`
      (:`then_0`
        (goto _label :!via `Reset`)))))

(event `self.ReceiveBeginPlay`
  (bind _npc (`self.NPC`))
  ;[1 1 1] Basic
  (bind _asbp_eco_character (cast `/Game/1GAME/Character/BP_EcoCharacter` (`GameplayStatics.GetPlayerCharacter` 0)))
  (set `self.As BP Eco Character` _asbp_eco_character)
  (`SceneComponent.SetVisibility` (`self.TextRender`) false false)
  (`KismetSystemLibrary.Delay` 0.2)
  (switch `/Game/1GAME/Character/NPC_List` (`self.NPC_List`)
    (:`NewEnumerator0`
      (`SkeletalMeshComponent.PlayAnimation` _npc "/Game/1GAME/Character/NPC_Animations/Idle_Anim.Idle_Anim" true))
    (:`NewEnumerator1`
      (`SkeletalMeshComponent.PlayAnimation` _npc "/Game/1GAME/Character/NPC_Animations/Idle_Anim.Idle_Anim" true))
    (:`NewEnumerator2`
      (`SkeletalMeshComponent.PlayAnimation` _npc "/Game/1GAME/Character/NPC_Animations/Idle_Anim.Idle_Anim" true))
    (:`NewEnumerator3`
      (`SkeletalMeshComponent.PlayAnimation` _npc "/Game/1GAME/Character/NPC_Animations/Idle_Anim.Idle_Anim" true))))

(event `Writter`
  ;[1 0.05967 0.1294] Display Dialogue
  ;;[1 0.1921 0] Dialogue 1
  (`/Engine/EditorBlueprintResources/StandardMacros.DoOnce` false :!label _label
    (:`Completed`
      (bind _returnvalue (`|CreateWidget` "/Game/1GAME/Information/ECOwritter_Widget.ECOwritter_Widget_C" (`GameplayStatics.GetPlayerController` 0) (`self.Chars Per Second`)))
      (bind _output_get (set `self.Current Widget` _returnvalue))
      (`UserWidget.AddToViewport` _output_get 0)
      (`/Game/1GAME/Information/ECOwritter_Widget.Write` _output_get (`self.Text To Speak`)))))

(event `EndText`
  ;[1 0.05967 0.1294] Display Dialogue
  (`Widget.RemoveFromParent` (`self.Current Widget`))
  (set `self.OnGoingTalk` false)
  (set `self.Finished` true)
  (`self.ResetOrder`)
  (`SkeletalMeshComponent.PlayAnimation` (`self.NPC`) "/Game/1GAME/Character/NPC_Animations/Idle_Anim.Idle_Anim" true))

(event `NextDialogue`
  ;[1 0.05967 0.1294] Display Dialogue
  ;;[1 0.1921 0] Dialogue 1
  (`self.ResetWritter`)
  (`self.SetNextText`))

(event `self.ReceiveActorEndOverlap`
  (params (OtherActor :type "Actor Object Reference"))
  ;[1 1 1] Basic
  (bind _asbp_eco_character (cast `/Game/1GAME/Character/BP_EcoCharacter` (`GameplayStatics.GetPlayerCharacter` 0)))
  (message `/Game/1GAME/Character/BPI_Interaction.Interact` _asbp_eco_character false self "")
  (set `self.As BP Eco Character` _asbp_eco_character)
  (`SceneComponent.SetVisibility` (`self.TextRender`) false false)
  (`self.EndText`)
  (`KismetSystemLibrary.Delay` 1.0)
  (set `self.Finished` false)
  (`self.ResetWritter`))

(event `self.ReceiveActorBeginOverlap`
  (params (OtherActor :type "Actor Object Reference"))
  ;[1 1 1] Basic
  (bind _asbp_eco_character (cast `/Game/1GAME/Character/BP_EcoCharacter` (`GameplayStatics.GetPlayerCharacter` 0)))
  (message `/Game/1GAME/Character/BPI_Interaction.Interact` _asbp_eco_character true self "")
  (set `self.As BP Eco Character` _asbp_eco_character)
  (`SceneComponent.SetVisibility` (`self.TextRender`) true false))

(event `NPCTalk`
  (params (NPCType :type Byte :default 0))
  ;[1 1 1] StartDialogueLogic
  (if (`self.Finished`)
    (`Widget.RemoveFromParent` (`self.Current Widget`))
    (`KismetSystemLibrary.Delay` 1.0)
    (set `self.Finished` false)
    (else
      (`KismetSystemLibrary.Delay` 0.2)
      (if (`self.OnGoingTalk`)
        (`self.NextDialogue`)
        (`Widget.RemoveFromParent` (`self.Current Widget`))
        (else
          (`/Engine/EditorBlueprintResources/StandardMacros.DoOnce` false :!label _label_2
            (:`Completed`
              (set `self.OnGoingTalk` true)
              (bind _asbp_eco_character (cast `/Game/1GAME/Character/BP_EcoCharacter` (`GameplayStatics.GetPlayerCharacter` 0)))
              (set `self.As BP Eco Character` _asbp_eco_character)
              (`self.SetNextText`)
              (`SkeletalMeshComponent.PlayAnimation` (`self.NPC`) "/Game/1GAME/Character/NPC_Animations/Head_Gesture.Head_Gesture" true)))))
      (`KismetSystemLibrary.Delay` 0.1)
      (if (not (`self.Finished`))
        (switch `/Game/1GAME/Character/NPC_List` (`self.NPC_List`)
          (:`NewEnumerator0`
            _)
          (:`NewEnumerator1`
            _)
          (:`NewEnumerator2`
            _)
          (:`NewEnumerator3`
            _))
        (`self.Writter`)))))

(event `SetNextText`
  ;[0 0.271 1] dIALOGUES
  ;;[1 0 0.03079] After collected
  (switch `/Game/1GAME/Character/NPC_List` (`self.NPC_List`)
    (:`NewEnumerator0`
      ;;[1 0.4684 0] Pescador
      (`|MultiGate` false :!label _label_3
        (:`Out 0`
          (set `self.Text To Speak` "Kelvin : Ah- Haru-san, welcome home!  \nIt’s been a while, you’ve grown so much… \nYou look great! \n"))
        (:`Out 1`
          (set `self.Text To Speak` "Kelvin : I’m sure your grandfather would be happy you came back. \nWe all miss Toji-san very much… \nBy the way, I’m pretty sure he left you something. \nAt your old place, I mean. You should check that out! \n"))
        (:`Out 2`
          (set `self.Text To Speak` "Kelvin :I don’t know much about it but… we can tell there’s something off about the island. \nIt’s messing with my sensors!! \nAnyhow, it’s nice seeing you again. We’re counting on you!"))
        (:`Out 3`
          (`self.EndText`))))
    (:`NewEnumerator1`
      ;;[0.2785 1 0] Fazendeiro
      (`|MultiGate` false :!label _label_4
        (:`Out 0`
          (set `self.Text To Speak` "Ah, Haru-san, welcome back… How can I be of service? \nThough… I must warn you.. . whatever has been spreading in the island, it’s been affecting the soil… \nSome of the other farmer bots on the other side of the island had entire crops ruined…"))
        (:`Out 1`
          (set `self.Text To Speak` "In fact, if you go to our farms, you might see some of the stuff \nWe should count ourselves lucky that it hasn’t completely ruined our farms yet.  \nDo you think you could help?"))
        (:`Out 2`
          (`self.EndText`)
          (bind _outactors (`GameplayStatics.GetAllActorsOfClass` "/Game/1GAME/Character/BP_PuzzleCamera.BP_PuzzleCamera_C"))
          (for _array_element _outactors
            (bind _asbp_puzzle_camera (cast `/Game/1GAME/Character/BP_PuzzleCamera` _array_element))
            (if (== (`/Game/1GAME/Character/BP_PuzzleCamera.CameraList` _asbp_puzzle_camera) 4)
              (`/Game/1GAME/Character/BP_PuzzleCamera.CameraStart` _asbp_puzzle_camera)
              (`KismetSystemLibrary.Delay` 4.0)
              (bind _outactors_2 (`GameplayStatics.GetAllActorsOfClass` "/Game/1GAME/Character/BP_PuzzleCamera.BP_PuzzleCamera_C"))
              (for _array_element_2 _outactors_2
                (bind _asbp_puzzle_camera_2 (cast `/Game/1GAME/Character/BP_PuzzleCamera` _array_element_2))
                (if (== (`/Game/1GAME/Character/BP_PuzzleCamera.CameraList` _asbp_puzzle_camera_2) 4)
                  (`/Game/1GAME/Character/BP_PuzzleCamera.CameraEnd` _asbp_puzzle_camera_2))))))))
    (:`NewEnumerator2`
      ;;[0.7029 1 0] Jardineiro
      (`|MultiGate` false :!label _label_5
        (:`Out 0`
          (set `self.Text To Speak` "Master Haru, as I live and breathe! \nWell, not quite, but… Welcome back!! \nI’ve been looking after your grandfather’s place, making sure weeds don't grow all over it…"))
        (:`Out 1`
          (set `self.Text To Speak` "Oh- I almost forgot- "))
        (:`Out 2`
          (set `self.Text To Speak` "Forgive me, my memory isn’t quite what it used to be… \nHe left you a recording. We didn’t listen to it but… \nI’m sure it’s important. It’s in his office. \nIt’s nice seeing you again!"))
        (:`Out 3`
          (`self.EndText`))))
    (:`NewEnumerator3`
      ;;[0.304 0.3646 0.2506] Mecanico
      (`|MultiGate` false :!label _label_6
        (:`Out 0`
          (set `self.Text To Speak` "Haru-san, welcome to my humble store! \nIs there anything I can do for you today? \nActually, there’s something I have to give you. \nToji-san left this with me before… you know…"))
        (:`Out 1`
          (set `self.Text To Speak` "it needed fixing so… Here it is!  \nYou should use it against those strange… pits.. puddles.. whatever they are \nEver since those things started popping up in the village my systems started going crazy! \nLucky I’m not in the farming business…"))
        (:`Out 2`
          (set `self.Text To Speak` "By the way, do you thing you could take a look at the wind power plant? we’ve been having some shortages… \nLet me know if anything need fixing!"))
        (:`Out 3`
          (`self.EndText`))))
    (:`NewEnumerator4`
      ;;[0.8802 0.3897 0] Macarronis
      (`|MultiGate` false
        (:`Out 0`
          (set `self.Text To Speak` "Kelvin : Ah- Haru-san, welcome home!  \nIt’s been a while, you’ve grown so much… \nYou look great! \n"))
        (:`Out 1`
          (set `self.Text To Speak` "Kelvin : I’m sure your grandfather would be happy you came back. \nWe all miss Toji-san very much… \nBy the way, I’m pretty sure he left you something. \nAt your old place, I mean. You should check that out! \n"))
        (:`Out 2`
          (set `self.Text To Speak` "Kelvin :I don’t know much about it but… we can tell there’s something off about the island. \nIt’s messing with my sensors!! \nAnyhow, it’s nice seeing you again. We’re counting on you!"))
        (:`Out 3`
          (`self.EndText`))))))

(event `AllowNext`
  ;[0 0.271 1] dIALOGUES
  ;;[1 0 0.03079] After collected
  (`/Engine/EditorBlueprintResources/StandardMacros.DoOnce` false :!via `Reset`))

(event `ResetOrder`
  ;[0 0.271 1] dIALOGUES
  ;;[1 0 0.03079] After collected
  (`|ExecutionSequence`
    (:`then_0`
      (goto _label_2 :!via `Reset`))
    (:`then_1`
      (goto _label_3 :!via `Reset`))
    (:`then_2`
      (goto _label_4 :!via `Reset`))
    (:`then_3`
      (goto _label_5 :!via `Reset`))
    (:`then_4`
      (goto _label_6 :!via `Reset`))))

(fn `UserConstructionScript`
  (bind _chapeu (`self.Chapeu`))
  (switch `/Game/1GAME/Character/NPC_List` (`self.NPC_List`)
    (:`NewEnumerator0`
      (bind _returnvalue (`AddComponent|NODE_AddSkeletalMeshComponent-0` :`RelativeTransform` (`KismetMathLibrary.MakeTransform` (0.0 0.0 0.0) (struct :`Roll` -90.0))))
      (set `self.Pescador` _returnvalue)
      (`StaticMeshComponent.SetStaticMesh` _chapeu "/Game/1GAME/Character/NPC_PESCADOR/buckethat_lp.buckethat_lp")
      (`PrimitiveComponent.SetMaterial` (`self.NPC`) 0 "/Game/1GAME/Character/NPC_PESCADOR/M_NPC_PESCADOR.M_NPC_PESCADOR")
      (`PrimitiveComponent.SetMaterial` _chapeu 0 "/Game/1GAME/Character/NPC_PESCADOR/M_bucket-hat_Unique.M_bucket-hat_Unique"))
    (:`NewEnumerator1`
      (bind _returnvalue_2 (`AddComponent|NODE_AddSkeletalMeshComponent-1` :`RelativeTransform` (`KismetMathLibrary.MakeTransform` (0.0 0.0 0.0) (struct :`Roll` -90.0))))
      (set `self.Fazendeiro` _returnvalue_2)
      (`StaticMeshComponent.SetStaticMesh` (`self.Chapeu`) "/Game/1GAME/Character/NPC_FAZENDEIRO/farmhat_lp.farmhat_lp")
      (`PrimitiveComponent.SetMaterial` (`self.NPC`) 0 "/Game/1GAME/Character/NPC_FAZENDEIRO/M_NPC_FAZENDEIRO.M_NPC_FAZENDEIRO")
      (`PrimitiveComponent.SetMaterial` (`self.Chapeu`) 0 "/Game/1GAME/Character/NPC_FAZENDEIRO/M_NPC_FAZENDEIRO.M_NPC_FAZENDEIRO"))
    (:`NewEnumerator2`
      (bind _returnvalue_3 (`AddComponent|NODE_AddSkeletalMeshComponent-6` :`RelativeTransform` (`KismetMathLibrary.MakeTransform` (0.0 0.0 0.0) (struct :`Roll` -90.0))))
      (set `self.Jardineiro` _returnvalue_3)
      (`StaticMeshComponent.SetStaticMesh` (`self.Chapeu`) "/Game/1GAME/Character/NPC_FAZENDEIRO/farmhat_lp.farmhat_lp")
      (`PrimitiveComponent.SetMaterial` (`self.NPC`) 0 "/Game/1GAME/Character/NPC_JARDINEIRO/M_JardineiroUnique.M_JardineiroUnique"))
    (:`NewEnumerator3`
      (bind _returnvalue_4 (`AddComponent|NODE_AddSkeletalMeshComponent-7` :`RelativeTransform` (`KismetMathLibrary.MakeTransform` (0.0 0.0 0.0) (struct :`Roll` -90.0))))
      (set `self.Mecanico` _returnvalue_4)
      (`StaticMeshComponent.SetStaticMesh` (`self.Chapeu`) "/Game/1GAME/Character/NPC_PESCADOR/buckethat_lp.buckethat_lp")
      (`PrimitiveComponent.SetMaterial` (`self.NPC`) 0 "/Game/1GAME/Character/NPC_MECANICO/M_MecanicoUnique.M_MecanicoUnique"))))
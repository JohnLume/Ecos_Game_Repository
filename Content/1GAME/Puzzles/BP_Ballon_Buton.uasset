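; Puzzle button for pumping balloons, offered as an interaction to BP_EcoCharacter on overlap.
; Each press plays sound and button animation and fills BP_Baloon actors tagged with its color, while a retriggerable delay clears the count after a brief pause.
; Ten rapid presses make those balloons fly (one-time), light up the button's material and notify every BP_Energy_Puzzle through BalonN.
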(event `ButtonPress`
  (params (Valvula :type "ActorComponent Object Reference"))
  ;[1 0 0.3907] Press
  (`|ExecutionSequence`
    (:`then_0`
      (bind _result (`/Engine/EditorBlueprintResources/StandardMacros.IncrementFloat` (`self.PressedAmount`))
        (:`  `
          (bind _output_get (set `self.PressedAmount` _result))
          (if (== _output_get 10.0)
            (`|ExecutionSequence`
              (:`then_0`
                (`/Engine/EditorBlueprintResources/StandardMacros.DoOnce` false
                  (:`Completed`
                    (bind _outactors (`GameplayStatics.GetAllActorsOfClass` "/Game/1GAME/Puzzles/BP_Baloon.BP_Baloon_C"))
                    (for _array_element _outactors
                      (if (`self.ActorHasTag` _array_element (`BlueprintGameplayTagLibrary.GetTagName` (`self.Color`)))
                        (bind _asbp_baloon (cast `/Game/1GAME/Puzzles/BP_Baloon` _array_element))
                        (`/Game/1GAME/Puzzles/BP_Baloon.FlyAnimation` _asbp_baloon)
                        (`GameplayStatics.SpawnSoundAtLocation` "/Game/1GAME/Sound/FX-INTERRUPTOR/SFX_EnergyOnC.SFX_EnergyOnC" (`self.K2_GetActorLocation`) (struct) 1.0 1.0 0.0 null null))))))
              (:`then_1`
                (`PrimitiveComponent.SetMaterial` (`self.Light`) 2 "/Game/1GAME/Puzzles/Hidro/Puzzle_Ligado.Puzzle_Ligado"))
              (:`then_2`
                (bind _outactors_2 (`GameplayStatics.GetAllActorsOfClass` "/Game/1GAME/Puzzles/BP_Energy_Puzzle.BP_Energy_Puzzle_C"))
                (for _array_element_2 _outactors_2
                  (bind _asbp_energy_puzzle (cast `/Game/1GAME/Puzzles/BP_Energy_Puzzle` _array_element_2))
                  (`/Game/1GAME/Puzzles/BP_Energy_Puzzle.BalonN` _asbp_energy_puzzle))))))))
    (:`then_1`
      (`KismetSystemLibrary.RetriggerableDelay` 0.3)
      (set `self.PressedAmount` 0.0))
    (:`then_2`
      (`self.Aesthetic`))
    (:`then_3`
      (`KismetSystemLibrary.Delay` 0.2)
      (bind _outactors_3 (`GameplayStatics.GetAllActorsOfClass` "/Game/1GAME/Puzzles/BP_Baloon.BP_Baloon_C"))
      (for _array_element_3 _outactors_3
        (if (`self.ActorHasTag` _array_element_3 (`BlueprintGameplayTagLibrary.GetTagName` (`self.Color`)))
          (bind _asbp_baloon_2 (cast `/Game/1GAME/Puzzles/BP_Baloon` _array_element_3))
          (`/Game/1GAME/Puzzles/BP_Baloon.FillBaloonAnim` _asbp_baloon_2))))))

(event `self.ReceiveBeginPlay`
  ;[1 0 0] Can press?
  (set `self.Org_Location` (`SceneComponent.K2_GetComponentLocation` (`self.Button`))))

(event `self.ReceiveActorBeginOverlap`
  (params (OtherActor :type "Actor Object Reference"))
  ;[1 0 0] Can press?
  (bind _asbp_eco_character (cast `/Game/1GAME/Character/BP_EcoCharacter` OtherActor))
  (message `/Game/1GAME/Character/BPI_Interaction.Interact` _asbp_eco_character true self ""))

(event `self.ReceiveActorEndOverlap`
  (params (OtherActor :type "Actor Object Reference"))
  ;[1 0 0] Can press?
  (bind _asbp_eco_character (cast `/Game/1GAME/Character/BP_EcoCharacter` OtherActor))
  (message `/Game/1GAME/Character/BPI_Interaction.Interact` _asbp_eco_character false self ""))

(event `Aesthetic`
  (bind _pressanimation (`self.PressAnimation`))
  (bind (_org_location_x _org_location_y _org_location_z) (`KismetMathLibrary.BreakVector` (`self.Org_Location`)))
  ;[0 0.1411 1] Visual
  (`|ExecutionSequence`
    (:`then_0`
      (`/Engine/EditorBlueprintResources/StandardMacros.DoOnce` false :!label _label
        (:`Completed`
          (`GameplayStatics.SpawnSoundAtLocation` "/Game/1GAME/Sound/Enchedor_Balao_Cue.Enchedor_Balao_Cue" (`self.K2_GetActorLocation`) (struct) 2.5 1.0 0.0 "/Game/1GAME/Sound/SFX_Atenutaion.SFX_Atenutaion" null)
          (`|ExecutionSequence`
            (:`then_0`
              (`KismetSystemLibrary.Delay` 0.3)
              (goto _label :!via `Reset`))))))
    (:`then_1`
      (`KismetSystemLibrary.Delay` 0.3)
      (`TimelineComponent.SetPlayRate` _pressanimation (/ 1.0 (`self.Duration`)))
      (`TimelineComponent.SetNewTime` _pressanimation (`self.StartOffset`))
      (bind (_direction _animationalpha) (`Timeline|PressAnimation`)
        (:`Update`
          (set `self.Alpha` _animationalpha)
          (`SceneComponent.K2_SetWorldLocation` (`self.Button`) (`KismetMathLibrary.MakeVector` _org_location_x _org_location_y (`KismetMathLibrary.Lerp` _org_location_z (+ _org_location_z 10.0) (`self.Alpha`))) false false))))))

(fn `UserConstructionScript`)
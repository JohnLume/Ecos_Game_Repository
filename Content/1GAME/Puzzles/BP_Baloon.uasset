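; Puzzle balloon actor that, when FlyAnimation is called, flies to a guide point and then floats there while its propeller spins.
; The SetFlight timeline moves the balloon using separate horizontal and vertical alpha curves, then hands off to the Floating timeline for vertical motion above the guide point.
; A parallel Rotation timeline rolls the propeller through full turns, with play rates and start offset driven by variables.
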(event `self.ReceiveBeginPlay`)

(event `FlyAnimation`
  (bind _rotation (`self.Rotation`))
  (bind _floating (`self.Floating`))
  (bind _set_flight (`self.Set Flight`))
  (bind (_original_location_x _original_location_y _original_location_z) (`KismetMathLibrary.BreakVector` (`self.Original location`)))
  (bind (_returnvalue_x _returnvalue_y _returnvalue_z) (`KismetMathLibrary.BreakVector` (`SceneComponent.K2_GetComponentLocation` (`self.GuidePoint`))))
  (bind (_returnvalue_x_2 _returnvalue_y_2 _returnvalue_z_2) (`KismetMathLibrary.BreakVector` (`SceneComponent.K2_GetComponentLocation` (`self.GuidePoint`))))
  (bind (_returnvalue_roll _returnvalue_pitch _returnvalue_yaw) (`KismetMathLibrary.BreakRotator` (`SceneComponent.K2_GetComponentRotation` (`self.balao_exp_helice`))))
  (`|ExecutionSequence`
    (:`then_0`
      (set `self.Original location` (`SceneComponent.K2_GetComponentLocation` (`self.Balao`)))
      (`TimelineComponent.SetPlayRate` _set_flight (/ 1.0 (`self.Duration_SetFlight`)))
      (`TimelineComponent.SetNewTime` _set_flight (`self.StartOffset`))
      (bind (_direction _x_alpha _z_alpha) (`Timeline|Set Flight`)
        (:`Update`
          (bind _output_get (set `self.Animation Alpha_SetFlight_X` _x_alpha))
          (bind _output_get_2 (set `self.Animation Alpha_SetFlight_Z` _z_alpha))
          (`SceneComponent.K2_SetWorldLocation` (`self.Balao`) (`KismetMathLibrary.MakeVector` (`KismetMathLibrary.Lerp` _original_location_x _returnvalue_x_2 _output_get) (`KismetMathLibrary.Lerp` _original_location_y _returnvalue_y_2 _output_get) (`KismetMathLibrary.Lerp` _original_location_z _returnvalue_z_2 _output_get_2)) false false))
        (:`Finished`
          ;[0.6979 0.7664 1] Floating
          (`TimelineComponent.SetPlayRate` _floating (/ 1.0 (`self.Duration`)))
          (`TimelineComponent.SetNewTime` _floating (`self.StartOffset`))
          (bind (_direction_2 _animationalpha) (`Timeline|Floating`)
            (:`Update`
              (set `self.Animation Alpha` _animationalpha)
              (`SceneComponent.K2_SetWorldLocation` (`self.Balao`) (`KismetMathLibrary.MakeVector` _returnvalue_x _returnvalue_y (`KismetMathLibrary.Lerp` _returnvalue_z (+ _returnvalue_z 200.0) (`self.Animation Alpha`))) false false))))))
    (:`then_2`
      ;[0.2193 0.237 1] Helice
      (`TimelineComponent.SetPlayRate` _rotation (`self.Duration_Helice`))
      (`TimelineComponent.SetNewTime` _rotation (`self.StartOffset`))
      (bind (_direction_3 _animationalpha_2) (`Timeline|Rotation`)
        (:`Update`
          (set `self.Animation Alpha_Helice` _animationalpha_2)
          (`SceneComponent.K2_SetWorldRotation` (`self.balao_exp_helice`) (`KismetMathLibrary.MakeRotator` (`KismetMathLibrary.Lerp` 0.0 360.0 (`self.Animation Alpha_Helice`)) _returnvalue_pitch _returnvalue_yaw) false false))))))

(fn `UserConstructionScript`)
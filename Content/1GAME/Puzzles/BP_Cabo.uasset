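; BP_Cabo is a spline-shaped cable for puzzles, with a point light that turns on when it is energized.
; The construction script builds one spline mesh per spline segment, storing only the last in Cabo.
; BeginPlay gives that last segment a dynamic material instance.
; The EneergiaOn event raises the light's intensity, while the material's Energy parameter write is disconnected and never runs.
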(event `self.ReceiveBeginPlay`
  (bind _returnvalue (`KismetMaterialLibrary.CreateDynamicMaterialInstance` null))
  (`PrimitiveComponent.SetMaterial` (`self.Cabo`) 0 _returnvalue))

(event `Eneergia On`
  (`LightComponent.SetIntensity` (`self.PointLight`) 100.0))

(fn `UserConstructionScript`
  (bind _spline (`self.Spline`))
  (for _index (range (`SplineComponent.GetNumberOfSplineSegments` _spline))
    (bind _returnvalue (`AddComponent|NODE_AddSplineMeshComponent-0`))
    (bind _output_get (set `self.Cabo` _returnvalue))
    (bind (_location _tangent) (`SplineComponent.GetLocationAndTangentAtSplinePoint` _spline _index "Local"))
    (bind (_location_2 _tangent_2) (`SplineComponent.GetLocationAndTangentAtSplinePoint` _spline (+ _index 1) "Local"))
    (`SplineMeshComponent.SetStartAndEnd` _output_get _location _tangent _location_2 _tangent_2 true)))
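; Interactable puzzle button that triggers energy puzzles of its color when pressed.
; Overlap begin and end tell BP_EcoCharacter, via InteractMessage, whether this button is available to interact with.
; ButtonPress calls ButtonPressed on every BP_Energy_Puzzle tagged with the button's color, then plays its feedback.
; The feedback plays a sound and a timeline yaw spin, guarded by a DoOnce until finished, with a FlipFlop alternating spin direction.
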(event `self.ReceiveActorBeginOverlap`
  (params (OtherActor :type "Actor Object Reference"))
  ;[1 0 0] Can press?
  (bind _asbp_eco_character (cast `/Game/1GAME/Character/BP_EcoCharacter` OtherActor))
  (message `/Game/1GAME/Character/BPI_Interaction.Interact` _asbp_eco_character true self ""))

(event `ButtonPress`
  (params (Valvula :type "ActorComponent Object Reference"))
  ;[1 0 0.3907] Press
  (`|ExecutionSequence`
    (:`then_0`
      (bind _outactors (`GameplayStatics.GetAllActorsOfClass` "/Game/1GAME/Puzzles/BP_Energy_Puzzle.BP_Energy_Puzzle_C"))
      (for _array_element _outactors
        (if (`self.ActorHasTag` _array_element (`BlueprintGameplayTagLibrary.GetTagName` (`self.Color`)))
          (bind _asbp_energy_puzzle (cast `/Game/1GAME/Puzzles/BP_Energy_Puzzle` _array_element))
          (`/Game/1GAME/Puzzles/BP_Energy_Puzzle.ButtonPressed` _asbp_energy_puzzle))))
    (:`then_2`
      (`self.Aesthetic`))))

(event `self.ReceiveActorEndOverlap`
  (params (OtherActor :type "Actor Object Reference"))
  ;[1 0 0] Can press?
  (bind _asbp_eco_character (cast `/Game/1GAME/Character/BP_EcoCharacter` OtherActor))
  (message `/Game/1GAME/Character/BPI_Interaction.Interact` _asbp_eco_character false self ""))

(event `Aesthetic`
  (bind _spinanimation (`self.SpinAnimation`))
  (bind (_returnvalue_roll _returnvalue_pitch _returnvalue_yaw) (`KismetMathLibrary.BreakRotator` (`SceneComponent.K2_GetComponentRotation` (`self.Button`))))
  ;[0 0.1411 1] Visual
  (`GameplayStatics.SpawnSound2D` null 1.0 1.0 0.0 null)
  (`/Engine/EditorBlueprintResources/StandardMacros.DoOnce` false :!label _label
    (:`Completed`
      (`TimelineComponent.SetPlayRate` _spinanimation (/ 1.0 (`self.Duration`)))
      (`TimelineComponent.SetNewTime` _spinanimation (`self.StartOffset`))
      (`|ExecutionSequence`
        (:`then_0`
          (bind (_direction _animationalpha) (`Timeline|SpinAnimation`)
            (:`Update`
              (set `self.Alpha` _animationalpha)
              (`SceneComponent.K2_SetWorldRotation` (`self.Button`) (`KismetMathLibrary.MakeRotator` _returnvalue_roll _returnvalue_pitch (`KismetMathLibrary.Lerp` _returnvalue_yaw (+ _returnvalue_yaw (`self.RotationAmount`)) (`self.Alpha`))) false false))
            (:`Finished`
              (goto _label :!via `Reset`))))
        (:`then_1`
          (`/Engine/EditorBlueprintResources/StandardMacros.FlipFlop`
            (:`A`
              (set `self.RotationAmount` 3.0))
            (:`B`
              (set `self.RotationAmount` -3.0))))))))

(fn `UserConstructionScript`)
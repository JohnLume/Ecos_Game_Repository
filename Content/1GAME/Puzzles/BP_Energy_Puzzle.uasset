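; BP_Energy_Puzzle is a puzzle actor that gains power after three triggers and then shows an on/off state on the Couchie component.
; BeginPlay sets an emissive material, and each BalonN call increments a counter that fires EnergyON at three, switching to the "Desligado" (off) material.
; ButtonPressed toggles Lit after a short delay, swapping between "Ligado" (on) and "Desligado" materials only once energy is on.
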(event `self.ReceiveBeginPlay`
  ;[1 0.4285 0] Litting
  (`PrimitiveComponent.SetMaterial` (`self.Couchie`) 2 "/Game/Basic/LevelPrototyping/Materials/M_Emissive.M_Emissive"))

(event `BalonN`
  ;[1 0.4285 0] Litting
  (bind _result (`/Engine/EditorBlueprintResources/StandardMacros.IncrementFloat` (`self.BalN`))
    (:`  `
      (bind _output_get (set `self.BalN` _result))
      (if (== _output_get 3.0)
        (`self.Energy ON`)))))

(event `Energy ON`
  ;[1 0.4285 0] Litting
  (set `self.Energy ON?` true)
  (`PrimitiveComponent.SetMaterial` (`self.Couchie`) 2 "/Game/1GAME/Puzzles/Hidro/Puzzle_Desligado.Puzzle_Desligado"))

(event `ButtonPressed`
  (bind _couchie (`self.Couchie`))
  (bind _energy_on_ (`self.Energy ON?`))
  ;[1 0.4285 0] Litting
  (`KismetSystemLibrary.Delay` 0.2)
  (bind _output_get (set `self.Lit` (not (`self.Lit`))))
  (if _output_get
    (if _energy_on_
      (`PrimitiveComponent.SetMaterial` _couchie 2 "/Game/1GAME/Puzzles/Hidro/Puzzle_Ligado.Puzzle_Ligado"))
    (elif _energy_on_
      (`PrimitiveComponent.SetMaterial` _couchie 2 "/Game/1GAME/Puzzles/Hidro/Puzzle_Desligado.Puzzle_Desligado"))))

(fn `UserConstructionScript`)
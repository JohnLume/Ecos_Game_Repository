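; BP_Hidropuzzle is a puzzle piece that toggles between lit and unlit material states when pressed.
; ButtonPressed waits briefly, flips the Lit flag and swaps one material slot on the Couchie mesh between the on and off materials.
; BeginPlay applies the off material when Lit starts true, without clearing the flag.
; The FireNargs activation and deactivation calls are disconnected and never run.
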(event `self.ReceiveBeginPlay`
  ;[1 0.4285 0] Litting
  (if (`self.Lit`)
    (`PrimitiveComponent.SetMaterial` (`self.Couchie`) 2 "/Game/1GAME/Puzzles/Puzzle_Desligado.Puzzle_Desligado")))

(event `ButtonPressed`
  (bind _couchie (`self.Couchie`))
  ;[1 0.4285 0] Litting
  (`KismetSystemLibrary.Delay` 0.2)
  (bind _output_get (set `self.Lit` (not (`self.Lit`))))
  (if _output_get
    (`PrimitiveComponent.SetMaterial` _couchie 2 "/Game/1GAME/Puzzles/Puzzle_Ligado.Puzzle_Ligado")
    (else
      (`PrimitiveComponent.SetMaterial` _couchie 2 "/Game/1GAME/Puzzles/Puzzle_Desligado.Puzzle_Desligado"))))

(fn `UserConstructionScript`)
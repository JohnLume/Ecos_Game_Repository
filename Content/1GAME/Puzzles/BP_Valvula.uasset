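; BP_Valvula is an interactable valve for the hydro puzzle, prompting BP_EcoCharacter to interact while overlapping it.
; ButtonPress calls ButtonPressed on every BP_Hidropuzzle actor tagged with the valve's color.
; It also flip-flops the light material between on and off, independently of puzzle state.
; A timeline-driven button movement with sound remains in the graph but never runs.
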(event `self.ReceiveActorBeginOverlap`
  (params (OtherActor :type "Actor Object Reference"))
  ;[1 0 0] Can press?
  (bind _asbp_eco_character (cast `/Game/1GAME/Character/BP_EcoCharacter` OtherActor))
  (message `/Game/1GAME/Character/BPI_Interaction.Interact` _asbp_eco_character true self ""))

(event `ButtonPress`
  (params (Valvula :type "ActorComponent Object Reference"))
  (bind _luz (`self.Luz`))
  ;[1 0 0.3907] Press
  (`|ExecutionSequence`
    (:`then_0`
      (bind _outactors (`GameplayStatics.GetAllActorsOfClass` "/Game/1GAME/Puzzles/BP_Hidropuzzle.BP_Hidropuzzle_C"))
      (for _array_element _outactors
        (if (`self.ActorHasTag` _array_element (`BlueprintGameplayTagLibrary.GetTagName` (`self.Color`)))
          (bind _asbp_hidropuzzle (cast `/Game/1GAME/Puzzles/BP_Hidropuzzle` _array_element))
          (`/Game/1GAME/Puzzles/BP_Hidropuzzle.ButtonPressed` _asbp_hidropuzzle))))
    (:`then_1`
      (`/Engine/EditorBlueprintResources/StandardMacros.FlipFlop`
        (:`A`
          (`PrimitiveComponent.SetMaterial` _luz 2 "/Game/1GAME/Puzzles/Puzzle_Ligado.Puzzle_Ligado"))
        (:`B`
          (`PrimitiveComponent.SetMaterial` _luz 2 "/Game/1GAME/Puzzles/Puzzle_Desligado.Puzzle_Desligado"))))))

(event `self.ReceiveActorEndOverlap`
  (params (OtherActor :type "Actor Object Reference"))
  ;[1 0 0] Can press?
  (bind _asbp_eco_character (cast `/Game/1GAME/Character/BP_EcoCharacter` OtherActor))
  (message `/Game/1GAME/Character/BPI_Interaction.Interact` _asbp_eco_character false self ""))

(event `Aesthetic`
  ;[0 0.1411 1] Visual
)

(fn `UserConstructionScript`)
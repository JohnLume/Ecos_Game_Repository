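; BP_Floating is a prop Blueprint that animates its Boiador component vertically to produce a floating motion.
; On BeginPlay it caches Boiador's world location and starts the Floating timeline, with play rate set by Duration and start time by StartOffset.
; Each update lerps only Z between LocationRef's current height and the original height using the timeline's alpha, keeping the original X and Y.
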(event `self.ReceiveBeginPlay`
  (bind _floating (`self.Floating`))
  (bind (_original_location_x _original_location_y _original_location_z) (`KismetMathLibrary.BreakVector` (`self.Original Location`)))
  (bind (_returnvalue_x _returnvalue_y _returnvalue_z) (`KismetMathLibrary.BreakVector` (`SceneComponent.K2_GetComponentLocation` (`self.LocationRef`))))
  ;[0.6979 0.7664 1] Floating
  (set `self.Original Location` (`SceneComponent.K2_GetComponentLocation` (`self.Boiador`)))
  (`TimelineComponent.SetPlayRate` _floating (/ 1.0 (`self.Duration`)))
  (`TimelineComponent.SetNewTime` _floating (`self.StartOffset`))
  (bind (_direction _animationalpha) (`Timeline|Floating`)
    (:`Update`
      (set `self.Animation Alpha` _animationalpha)
      (`SceneComponent.K2_SetWorldLocation` (`self.Boiador`) (`KismetMathLibrary.MakeVector` _original_location_x _original_location_y (`KismetMathLibrary.Lerp` _returnvalue_z _original_location_z (`self.Animation Alpha`))) false false))))

(fn `UserConstructionScript`)
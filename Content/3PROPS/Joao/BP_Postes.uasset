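; BP_Postes is a lamp post prop with a point light that is either lit or off, based on its Lit flag.
; When lit, it applies LightIntensity and the glowing lantern material to the Poster mesh; otherwise it zeroes the light and applies the off material.
; The construction script applies this state at edit time, and the PostesOn event repeats the same logic so the state can be refreshed at runtime.
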(event `PostesOn`
  (if (`self.Lit?`)
    (`LightComponent.SetIntensity` (`self.PointLight`) (`self.Light Intensity`))
    (`PrimitiveComponent.SetMaterial` (`self.Poster`) 2 "/Game/1GAME/Puzzles/Solar/M_Lantern_Poste.M_Lantern_Poste")
    (else
      (`LightComponent.SetIntensity` (`self.PointLight`) 0.0)
      (`PrimitiveComponent.SetMaterial` (`self.Poster`) 2 "/Game/1GAME/Puzzles/Solar/M_Lantern_Off.M_Lantern_Off"))))

(fn `UserConstructionScript`
  (if (`self.Lit?`)
    (`LightComponent.SetIntensity` (`self.PointLight`) (`self.Light Intensity`))
    (`PrimitiveComponent.SetMaterial` (`self.Poster`) 2 "/Game/1GAME/Puzzles/Solar/M_Lantern_Poste.M_Lantern_Poste")
    (else
      (`LightComponent.SetIntensity` (`self.PointLight`) 0.0)
      (`PrimitiveComponent.SetMaterial` (`self.Poster`) 2 "/Game/1GAME/Puzzles/Solar/M_Lantern_Off.M_Lantern_Off"))))